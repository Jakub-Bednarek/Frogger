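; Finish line actor for the Frogger kart track that counts each BP_FroggiKart's laps on overlap.
; A crossing with valid track progress adds a lap; one without subtracts a lap, gated by a shared DoOnce that valid crossings can reset.
; For the player, it prints the count and fires OnLapProgress below four laps, otherwise disables input and shows the W_WIn widget after a short delay.
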(event `self.ReceiveActorBeginOverlap`
  (params (OtherActor :type "Actor Object Reference"))
  (bind _asbp_froggi_kart (cast `/Game/Frogger/Level_3_Content/FroggiKartPlayer/BP_FroggiKart` OtherActor))
  (if (`/Game/Frogger/Level_3_Content/FroggiKartPlayer/BP_FroggiKart.GetTrackProgress` _asbp_froggi_kart)
    (bind _laps (`/Game/Frogger/Level_3_Content/FroggiKartPlayer/BP_FroggiKart.Laps` _asbp_froggi_kart))
    (bind _result (`/Engine/EditorBlueprintResources/StandardMacros.IncrementInt` _laps)
      (:`  `
        (if (== _asbp_froggi_kart (`GameplayStatics.GetPlayerPawn` 0))
          (`KismetSystemLibrary.PrintString` (`KismetStringLibrary.Conv_IntToString` _laps) true true (struct :`G` 0.66 :`B` 1.0 :`A` 1.0) 4000000000.0)
          (if (< _laps 4)
            (`self.OnLapProgress` _result)
            (goto _label :!via `Reset`)
            (else
              (`KismetSystemLibrary.PrintString` "koniec" true true (struct :`R` 0.263747 :`B` 1.0 :`A` 1.0) 1000.0)
              (`self.DisableInput` _asbp_froggi_kart (`PlayerState.GetPlayerController` (`Pawn.PlayerState` _asbp_froggi_kart)))
              (`KismetSystemLibrary.Delay` 2.0)
              (bind _returnvalue (`|CreateWidget` "/Game/Frogger/Level_3_Content/UI/W_WIn.W_WIn_C"))
              (`UserWidget.AddToViewport` _returnvalue 0)))
          (else
            (goto _label :!via `Reset`)))))
    (else
      (`/Engine/EditorBlueprintResources/StandardMacros.DoOnce` false :!label _label
        (:`Completed`
          (`/Engine/EditorBlueprintResources/StandardMacros.DecrementInt` (`/Game/Frogger/Level_3_Content/FroggiKartPlayer/BP_FroggiKart.Laps` _asbp_froggi_kart)))))))

(fn `UserConstructionScript`)