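; Physics-driven racing kart pawn for FroggiRacer that registers with the game mode and serves as both player and AI racer.
; Four per-wheel line traces apply spring suspension, while forces and yaw torque on the Box drive and steer it.
; Enhanced Input drives the player, while karts not possessed by player 0 derive throttle and steering from BP_TrackSpline directions.
; The spline also yields lap-based progress and the timed reset position after toppling.
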(event `self.ReceiveBeginPlay`
  (bind _returnvalue (`GameplayStatics.GetActorOfClass` "/Game/Frogger/Level_3_Content/Track/BP_TrackSpline.BP_TrackSpline_C"))
  (set `self.Track` _returnvalue)
  (bind _returnvalue_2 (`|CreateWidget` "/Game/Frogger/Level_3_Content/UI/W_HUD.W_HUD_C"))
  (`UserWidget.AddToViewport` _returnvalue_2 0)
  (bind _asgm_froggi_racer (cast `/Game/Frogger/Level_3_Content/FroggiKartPlayer/GM_FroggiRacer` (`GameplayStatics.GetGameMode`)))
  (`/Game/Frogger/Level_3_Content/FroggiKartPlayer/GM_FroggiRacer.AddKart` _asgm_froggi_racer self)
  (`EnhancedInputSubsystemInterface.AddMappingContext` (pcsubsystem `EnhancedInputLocalPlayerSubsystem` (`GameplayStatics.GetPlayerController` 0)) "/Game/Frogger/Level_3_Content/FroggiKartPlayer/Inputs/IMC_Vehicle.IMC_Vehicle" 0 (struct)))

(event `self.ReceiveTick`
  (params (DeltaSeconds :type "Float (single-precision)"))
  (`|ExecutionSequence`
    (:`then_0`
      (`self.SuspensionCast` (`self.FL_Wheel`))
      (`self.SuspensionCast` (`self.FR_Wheel`))
      (`self.SuspensionCast` (`self.BR_Wheel`))
      (`self.SuspensionCast` (`self.BL_Wheel`))
      (`self.CalculateAcceleration`)
      (`self.IsToppled`))
    (:`then_1`
      (if (!= (`self.GetController`) (`GameplayStatics.GetPlayerController` 0))
        (`self.AI_Acceleration` (`self.GetAIThrottle`))
        (`self.AI_SteerKart` (`self.GetAISteering`))))))

(event `EnhancedInput|/Game/Frogger/Level_3_Content/FroggiKartPlayer/Inputs/IA_Accelerate`
  (params (ActionValue :type "Float (double-precision)") (ElapsedSeconds :type "Float (double-precision)") (TriggeredSeconds :type "Float (double-precision)") (InputAction :type "InputAction Object Reference" :default "/Game/Frogger/Level_3_Content/FroggiKartPlayer/Inputs/IA_Accelerate.IA_Accelerate"))
  (:`Triggered`
    (set `self.AccelerationInput` (`KismetMathLibrary.FInterpTo` (`self.AccelerationInput`) (`KismetMathLibrary.SelectFloat` ActionValue (`self.AccelerationInput`) (`self.IsOnGround`)) (`GameplayStatics.GetWorldDeltaSeconds`) 0.5))))

(event `EnhancedInput|/Game/Frogger/Level_3_Content/FroggiKartPlayer/Inputs/IA_Steer`
  (params (ActionValue :type "Float (double-precision)") (ElapsedSeconds :type "Float (double-precision)") (TriggeredSeconds :type "Float (double-precision)") (InputAction :type "InputAction Object Reference" :default "/Game/Frogger/Level_3_Content/FroggiKartPlayer/Inputs/IA_Steer.IA_Steer"))
  (bind (_relativerotation_roll _relativerotation_pitch _relativerotation_yaw) (`KismetMathLibrary.BreakRotator` (`SceneComponent.RelativeRotation` (`self.FL_Wheel`))))
  (:`Triggered`
    (`PrimitiveComponent.AddTorqueInRadians` (`self.Box`) (`KismetMathLibrary.MakeVector` 0.0 0.0 (* ActionValue 12000000.0 (`self.AccelerationInput`))) "None" false)
    (`SceneComponent.K2_SetRelativeRotation` (`self.FL_Wheel`) (`KismetMathLibrary.MakeRotator` 0.0 0.0 (`KismetMathLibrary.FInterpTo` _relativerotation_yaw (* ActionValue 50.0) (`GameplayStatics.GetWorldDeltaSeconds`) 3.0)) false false)
    (`SceneComponent.K2_SetRelativeRotation` (`self.FR_Wheel`) (`KismetMathLibrary.MakeRotator` 0.0 0.0 (`KismetMathLibrary.FInterpTo` _relativerotation_yaw (* ActionValue 50.0) (`GameplayStatics.GetWorldDeltaSeconds`) 3.0)) false false))
  (:`Completed`
    (`SceneComponent.K2_SetRelativeRotation` (`self.FL_Wheel`) (`KismetMathLibrary.MakeRotator` 0.0 0.0 (`KismetMathLibrary.FInterpTo` 0.0 0.0 (`GameplayStatics.GetWorldDeltaSeconds`) 20.0)) false false)
    (`SceneComponent.K2_SetRelativeRotation` (`self.FR_Wheel`) (`KismetMathLibrary.MakeRotator` 0.0 0.0 (`KismetMathLibrary.FInterpTo` 0.0 0.0 (`GameplayStatics.GetWorldDeltaSeconds`) 20.0)) false false)))

(fn `AccelerateKart`
  (params (WheelComp :type "SceneComponent Object Reference"))
  (bind _box (`self.Box`))
  (`PrimitiveComponent.AddForceAtLocation` (`self.Box`) (+ (* (`SceneComponent.GetForwardVector` _box) 1000.0 (`self.AccelerationInput`) (`PrimitiveComponent.GetMass` _box)) (`KismetMathLibrary.SelectVector` (0.0 0.0 0.0) (0.0 0.0 -1000.0) (`self.IsOnGround`))) (`SceneComponent.K2_GetComponentLocation` WheelComp) "None")
  (`PrimitiveComponent.SetCenterOfMass` (`self.Box`) (* (30.0 0.0 0.0) (`self.AccelerationInput`)) "None"))

(fn `AI_Acceleration`
  (params (Throttle :type "Float (double-precision)"))
  (set `self.AccelerationInput` (`KismetMathLibrary.FInterpTo` (`self.AccelerationInput`) (`KismetMathLibrary.SelectFloat` Throttle (`self.AccelerationInput`) (`self.IsOnGround`)) (`GameplayStatics.GetWorldDeltaSeconds`) 0.8)))

(fn `AI_SteerKart`
  (params (A :type "Float (double-precision)"))
  (bind (_relativerotation_roll _relativerotation_pitch _relativerotation_yaw) (`KismetMathLibrary.BreakRotator` (`SceneComponent.RelativeRotation` (`self.FL_Wheel`))))
  (`PrimitiveComponent.AddTorqueInRadians` (`self.Box`) (`KismetMathLibrary.MakeVector` 0.0 0.0 (* A 15500000.0 (* (`self.AccelerationInput`) 2.0))) "None" false)
  (`SceneComponent.K2_SetRelativeRotation` (`self.FL_Wheel`) (`KismetMathLibrary.MakeRotator` 0.0 0.0 (`KismetMathLibrary.FInterpTo` _relativerotation_yaw A (`GameplayStatics.GetWorldDeltaSeconds`) 3.0)) false false)
  (`SceneComponent.K2_SetRelativeRotation` (`self.FR_Wheel`) (`KismetMathLibrary.MakeRotator` 0.0 0.0 (`KismetMathLibrary.FInterpTo` _relativerotation_yaw A (`GameplayStatics.GetWorldDeltaSeconds`) 3.0)) false false))

(fn `CalculateAcceleration`
  (bind _accelerationinput (`self.AccelerationInput`))
  (bind _output_get (set `self.Acceleration` (* (`KismetMathLibrary.Lerp` 0.0 150000.0 _accelerationinput) _accelerationinput)))
  (set `self.AccelerationInput` (`KismetMathLibrary.FInterpTo` (`self.AccelerationInput`) 0.0 (`GameplayStatics.GetWorldDeltaSeconds`) 0.3))
  (`SceneComponent.K2_AddLocalRotation` (`self.Wheel_BL`) (`KismetMathLibrary.MakeRotator` 0.0 (/ _output_get -10000.0)) false false)
  (`SceneComponent.K2_AddLocalRotation` (`self.Wheel_BR`) (`KismetMathLibrary.MakeRotator` 0.0 (/ _output_get -10000.0)) false false)
  (`SceneComponent.K2_AddLocalRotation` (`self.Wheel_FR`) (`KismetMathLibrary.MakeRotator` 0.0 (/ _output_get -10000.0)) false false)
  (`SceneComponent.K2_AddLocalRotation` (`self.Wheel_FL`) (`KismetMathLibrary.MakeRotator` 0.0 (/ _output_get -10000.0)) false false))

(fn `GetAISteering`
  (returns (ReturnValue :type "Float (double-precision)"))
  (bind _returnvalue (`KismetMathLibrary.Dot_VectorVector` (`SplineComponent.FindDirectionClosestToWorldLocation` (`/Game/Frogger/Level_3_Content/Track/BP_TrackSpline.Spline` (`self.Track`)) (+ (`self.K2_GetActorLocation`) (* (`self.GetActorForwardVector`) 500.0)) "World") (`self.GetActorRightVector`)))
  (return (* (`KismetMathLibrary.MultiplyMultiply_FloatFloat` (+ (`KismetMathLibrary.Abs` _returnvalue) 2.5) 3.0) _returnvalue (`self.AccelerationInput`))))

(fn `GetAIThrottle`
  (returns (ReturnValue :type "Float (double-precision)"))
  (bind _returnvalue (`KismetMathLibrary.Dot_VectorVector` (`SplineComponent.FindDirectionClosestToWorldLocation` (`/Game/Frogger/Level_3_Content/Track/BP_TrackSpline.Spline` (`self.Track`)) (`self.K2_GetActorLocation`) "World") (`self.GetActorForwardVector`)))
  (return (* (`KismetMathLibrary.FClamp` (`KismetMathLibrary.Abs` _returnvalue) 0.4) (`KismetMathLibrary.SignOfFloat` _returnvalue))))

(fn `GetCourseProgress`
  (returns (ReturnValue :type "Float (double-precision)"))
  (bind _track (`self.Track`))
  (bind _spline (`/Game/Frogger/Level_3_Content/Track/BP_TrackSpline.Spline` _track))
  (return (+ (/ (`SplineComponent.GetDistanceAlongSplineAtLocation` _spline (`SplineComponent.FindLocationClosestToWorldLocation` (`/Game/Frogger/Level_3_Content/Track/BP_TrackSpline.Spline` _track) (`self.K2_GetActorLocation`) "World") "World") (`SplineComponent.GetSplineLength` _spline)) (`self.Laps`))))

(fn `GetTrackProgress`
  (returns (IsCorrectDirection :type Boolean))
  (return (> (`KismetMathLibrary.Dot_VectorVector` (`SplineComponent.FindDirectionClosestToWorldLocation` (`/Game/Frogger/Level_3_Content/Track/BP_TrackSpline.Spline` (`self.Track`)) (`self.K2_GetActorLocation`) "World") (`KismetMathLibrary.Normal` (`self.GetVelocity`))) 0.0)))

(fn `IsOnGround`
  (returns (ReturnValue :type Boolean))
  (bind _returnvalue (`self.K2_GetActorLocation`))
  (bind (_outhit _returnvalue_2) (`KismetSystemLibrary.LineTraceSingle` _returnvalue (- _returnvalue (0.0 0.0 30.0)) "TraceTypeQuery1"))
  (return _returnvalue_2))

(fn `IsToppled`
  (if (and (< (`KismetMathLibrary.Dot_VectorVector` (`self.GetActorUpVector`) (0.0 0.0 1.0)) 0.8) (not (`KismetSystemLibrary.K2_IsValidTimerHandle` (`self.ResetTimer`))))
    (bind _returnvalue (`KismetSystemLibrary.K2_SetTimerDelegate` (`|CreateDelegate` :!event `Reset Position`) 3.0))
    (set `self.ResetTimer` _returnvalue)))

(fn `Reset Position`
  (bind _returnvalue (`self.K2_GetActorLocation`))
  (bind _spline (`/Game/Frogger/Level_3_Content/Track/BP_TrackSpline.Spline` (`self.Track`)))
  (`KismetSystemLibrary.K2_ClearAndInvalidateTimerHandle` (`self.ResetTimer`))
  (`self.K2_SetActorLocationAndRotation` (`SplineComponent.FindLocationClosestToWorldLocation` _spline _returnvalue "World") (`KismetMathLibrary.Conv_VectorToRotator` (`SplineComponent.FindDirectionClosestToWorldLocation` _spline _returnvalue "World")))
  (set `self.AccelerationInput` 0.0))

(fn `SuspensionCast`
  (params (`Wheels Comp` :type "SceneComponent Object Reference"))
  (bind _returnvalue (`SceneComponent.K2_GetComponentLocation` `Wheels Comp`))
  (bind _returnvalue_2 (`SceneComponent.GetChildComponent` (`local.Wheels Comp`) 0))
  (bind (_relativelocation_x _relativelocation_y _relativelocation_z) (`KismetMathLibrary.BreakVector` (`SceneComponent.RelativeLocation` _returnvalue_2)))
  (bind _outhit (`KismetSystemLibrary.LineTraceSingle` :`Start` _returnvalue :`End` (+ _returnvalue (* (`SceneComponent.GetUpVector` `Wheels Comp`) -60.0)) :`TraceChannel` "TraceTypeQuery1" :`DrawDebugType` "ForOneFrame"))
  (bind (_bblockinghit _binitialoverlap _time _distance _location _impactpoint _normal _impactnormal _physmat _hitactor _hitcomponent _hitbonename _bonename _hititem _elementindex _faceindex _tracestart _traceend) (`GameplayStatics.BreakHitResult` _outhit))
  (if _bblockinghit
    (`PrimitiveComponent.AddForceAtLocation` (`self.Box`) (* (- 1.0 (`KismetMathLibrary.NormalizeToRange` _distance 0.0 60.0)) (`KismetMathLibrary.GetDirectionUnitVector` _traceend _tracestart) 80000.0) (`SceneComponent.K2_GetComponentLocation` (`local.Wheels Comp`)) "None")
    (`self.AccelerateKart` (`local.Wheels Comp`))
    (`SceneComponent.K2_SetRelativeLocation` _returnvalue_2 (`KismetMathLibrary.MakeVector` 0.0 0.0 (`KismetMathLibrary.FInterpTo` _relativelocation_z (+ (* _distance -1.0) 25.0) (`GameplayStatics.GetWorldDeltaSeconds`) 3.0)) false false)
    (else
      (`self.AccelerateKart` (`local.Wheels Comp`)))))

(fn `UserConstructionScript`
  (bind _returnvalue (`PrimitiveComponent.CreateDynamicMaterialInstance` (`self.Cube`) 0 "/Game/Frogger/Level_3_Content/FroggiKartPlayer/M_KartBody_Inst.M_KartBody_Inst" "None"))
  (`MaterialInstanceDynamic.SetVectorParameterValue` _returnvalue "Color" (`self.DebugColor`))
  (`PrimitiveComponent.SetMaterial` (`self.Cube`) 0 _returnvalue))