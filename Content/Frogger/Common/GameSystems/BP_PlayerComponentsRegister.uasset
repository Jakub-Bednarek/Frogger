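; BP_PlayerComponentsRegister is an actor that registers player component sets for the levels of the Frogger game.
; On BeginPlay, RegisterComponents registers a default component set, then one component set for each of six test levels.
; A CreateDefaults flag on each level's registration is enabled for every level except the third.
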(event `self.ReceiveBeginPlay`
  (`self.RegisterComponents`))

(fn `RegisterComponents`
  (`self.RegisterDefaultComponents` (`self.DefaultComponents`))
  (`self.RegisterLevelComponentsSet` "/Game/Frogger/Maps/TestLevel_1/TestLevel_1.TestLevel_1" (`self.FirstLevelComponents`))
  (`self.RegisterLevelComponentsSet` "/Game/Frogger/Maps/TestLevel_2/TestLevel_2.TestLevel_2" (`self.SecondLevelComponents`))
  (`self.RegisterLevelComponentsSet` "/Game/Frogger/Maps/TestLevel_3/TestLevel_3.TestLevel_3" (`self.ThirdLevelComponents`) false)
  (`self.RegisterLevelComponentsSet` "/Game/Frogger/Maps/TestLevel_4/TestLevel_4.TestLevel_4" (`self.FourthLevelComponents`))
  (`self.RegisterLevelComponentsSet` "/Game/Frogger/Maps/TestLevel_5/TestLevel_5.TestLevel_5" (`self.FifthLevelComponents`))
  (`self.RegisterLevelComponentsSet` "/Game/Frogger/Maps/TestLevel_6/TestLevel_6.TestLevel_6" (`self.SixthLevelComponents`)))

(fn `UserConstructionScript`)