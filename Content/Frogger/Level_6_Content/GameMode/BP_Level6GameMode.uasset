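; BP_Level6GameMode is the game mode for Frogger Level 6.
; On BeginPlay it deletes the Level6Slot save, and HandleStartingNewPlayer only calls the parent implementation.
; A disconnected chain would load that save, find a PlayerStart by its SpawnTag, then spawn and possess a BP_ThirdPersonCharacter_Child there, but it never runs.
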(event `self.ReceiveBeginPlay`
  (`GameplayStatics.DeleteGameInSlot` "Level6Slot"))

(event `self.HandleStartingNewPlayer`
  (params (NewPlayer :type "PlayerController Object Reference"))
  (`parent.HandleStartingNewPlayer` NewPlayer))

(fn `UserConstructionScript`)