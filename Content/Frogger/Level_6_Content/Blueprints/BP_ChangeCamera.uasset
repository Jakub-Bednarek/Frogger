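; Trigger actor in Frogger Level 6 that switches the player's view to a level camera while the third-person character is inside it.
; On begin overlap it blends player 0's view to the first BP_Camera found in the level and blocks the character's rotation.
; On end overlap it blends the view back to the character and allows rotation again.
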(event `self.ReceiveActorBeginOverlap`
  (params (OtherActor :type "Actor Object Reference"))
  (bind _asbp_third_person_character_child (cast `/Game/Frogger/Level_6_Content/Blueprints/BP_ThirdPersonCharacter_Child` OtherActor))
  (if (== _asbp_third_person_character_child OtherActor)
    (bind _outactors (`GameplayStatics.GetAllActorsOfClass` "/Game/Frogger/Level_6_Content/Blueprints/BP_Camera.BP_Camera_C"))
    (`PlayerController.SetViewTargetWithBlend` (`GameplayStatics.GetPlayerController` 0) (`|GetArrayItem` _outactors) 0.5 "VTBlend_Linear" 0.0 false)
    (`/Game/Frogger/Level_6_Content/Blueprints/BP_ThirdPersonCharacter_Child.BlockRotation` _asbp_third_person_character_child)))

(event `self.ReceiveActorEndOverlap`
  (params (OtherActor :type "Actor Object Reference"))
  (bind _asbp_third_person_character_child (cast `/Game/Frogger/Level_6_Content/Blueprints/BP_ThirdPersonCharacter_Child` OtherActor))
  (`PlayerController.SetViewTargetWithBlend` (`GameplayStatics.GetPlayerController` 0) _asbp_third_person_character_child 0.5 "VTBlend_Linear" 0.0 false)
  (`/Game/Frogger/Level_6_Content/Blueprints/BP_ThirdPersonCharacter_Child.AllowRotation` _asbp_third_person_character_child))

(fn `UserConstructionScript`)