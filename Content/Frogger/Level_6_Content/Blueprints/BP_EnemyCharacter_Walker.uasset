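; Walking wolf enemy for Frogger Level 6 that chases and attacks the player, extending a parent enemy's detection and attack logic.
; While detection passes on Tick, it moves toward the player and attacks on arrival with a cooldown; otherwise it stops.
; Attack, hit and death flags are set on ABP_Wolf; being hit or dead suppresses detection, and being hit also blocks further damage.
; Death destroys the actor after a delay.
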(event `self.ReceiveTick`
  (params (DeltaSeconds :type "Float (single-precision)"))
  (`parent.ReceiveTick` 0.0)
  (bind _detect (`self.DetectPlayer`))
  (if _detect
    (`|AIMoveTo` self (0.0 0.0 0.0) (`GameplayStatics.GetPlayerCharacter` 0) 180.0 true
      (:`OnSuccess`
        (`/Engine/EditorBlueprintResources/StandardMacros.DoOnce` false :!label _label
          (:`Completed`
            (`self.Attack`)
            (`KismetSystemLibrary.Delay` 2.0)
            (goto _label :!via `Reset`)))))
    (else
      (`MovementComponent.StopMovementImmediately` (`self.CharacterMovement`)))))

(event `self.Attack`
  (`/Engine/EditorBlueprintResources/StandardMacros.DoOnce` false :!label _label_2
    (:`Completed`
      (bind _asabp_wolf (cast `/Game/Frogger/Level_6_Content/Animation/ABP_Wolf` (`SkeletalMeshComponent.GetAnimInstance` (`self.Mesh`))))
      (set `/Game/Frogger/Level_6_Content/Animation/ABP_Wolf.isAttacking` true _asabp_wolf)
      (`parent.Attack`)
      (`KismetSystemLibrary.Delay` 1.0)
      (set `/Game/Frogger/Level_6_Content/Animation/ABP_Wolf.isAttacking` false _asabp_wolf)
      (goto _label_2 :!via `Reset`))))

(event `Hit`
  (params (Damage :type "Float (double-precision)"))
  (bind _asabp_wolf (cast `/Game/Frogger/Level_6_Content/Animation/ABP_Wolf` (`SkeletalMeshComponent.GetAnimInstance` (`self.Mesh`))))
  (if (not (`/Game/Frogger/Level_6_Content/Animation/ABP_Wolf.isHit` _asabp_wolf))
    (bind _output_get (set `self.Health` (- (`self.Health`) Damage)))
    (if (<= _output_get 0.0)
      (set `/Game/Frogger/Level_6_Content/Animation/ABP_Wolf.isDead` true _asabp_wolf)
      (`KismetSystemLibrary.Delay` 10.0)
      (`self.K2_DestroyActor`)
      (else
        (set `/Game/Frogger/Level_6_Content/Animation/ABP_Wolf.isHit` true _asabp_wolf)))))

(fn `DetectPlayer`
  (returns (Detect :type Boolean))
  (bind _detect (`parent.DetectPlayer`))
  (bind _asabp_wolf (cast `/Game/Frogger/Level_6_Content/Animation/ABP_Wolf` (`SkeletalMeshComponent.GetAnimInstance` (`self.Mesh`))))
  (return (and (not (or (`/Game/Frogger/Level_6_Content/Animation/ABP_Wolf.isHit` _asabp_wolf) (`/Game/Frogger/Level_6_Content/Animation/ABP_Wolf.isDead` _asabp_wolf))) _detect)))

(fn `UserConstructionScript`
  (`parent.UserConstructionScript`))