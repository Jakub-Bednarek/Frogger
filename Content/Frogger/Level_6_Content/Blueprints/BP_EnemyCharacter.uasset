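; BP_EnemyCharacter is an enemy character for Frogger Level 6 that can detect and damage the player.
; DetectPlayer returns whether the player pawn is closer to the enemy's mesh than SeeRange, using a plain distance check.
; The Attack event casts the player to BP_ThirdPersonCharacter_Child and calls its Hit with Damage as non-water damage, without checking range.
; Its own Hit event and Tick are empty, and nothing here calls Attack or DetectPlayer.
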(event `self.ReceiveTick`
  (params (DeltaSeconds :type "Float (single-precision)")))

(event `Attack`
  (bind _asbp_third_person_character_child (cast `/Game/Frogger/Level_6_Content/Blueprints/BP_ThirdPersonCharacter_Child` (`GameplayStatics.GetPlayerCharacter` 0)))
  (`/Game/Frogger/Level_6_Content/Blueprints/BP_ThirdPersonCharacter_Child.Hit` _asbp_third_person_character_child (`self.Damage`) false))

(event `Hit`
  (params (Damage :type "Float (double-precision)")))

(fn `DetectPlayer`
  (returns (Detect :type Boolean))
  (return (< (`KismetMathLibrary.VSize` (- (`SceneComponent.K2_GetComponentLocation` (`self.Mesh`)) (`self.K2_GetActorLocation` (`GameplayStatics.GetPlayerPawn` 0)))) (`self.seeRange`))))

(fn `UserConstructionScript`)