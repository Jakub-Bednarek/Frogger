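; Moving lily for Frogger Level 6 that shuttles its AshooFlower component back and forth between the Left and Right markers.
; BeginPlay caches both markers' relative locations as movement targets.
; Tick uses two DoOnce gates, selected by IsLeft, to run a timed MoveComponentTo, wait, flip direction and reset the gate.
; An alternative MoveLily graph with a fixed move duration is never run.
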(event `self.ReceiveBeginPlay`
  (set `self.isLeft` true)
  (set `self.LocationRight` (`KismetMathLibrary.TransformLocation` (`SceneComponent.GetRelativeTransform` (`self.Right`))))
  (set `self.LocationLeft` (`KismetMathLibrary.TransformLocation` (`SceneComponent.GetRelativeTransform` (`self.Left`)))))

(event `self.ReceiveTick`
  (params (DeltaSeconds :type "Float (single-precision)"))
  (bind _ashoo_flower (`self.ashoo_flower`))
  (bind _timetodestination (`self.TimeToDestination`))
  (if (`self.isLeft`)
    (`/Engine/EditorBlueprintResources/StandardMacros.DoOnce` false :!label _label
      (:`Completed`
        (`KismetSystemLibrary.MoveComponentTo` _ashoo_flower (`self.LocationRight`) (struct) false false _timetodestination)
        (`KismetSystemLibrary.Delay` (`self.Wait`))
        (set `self.isLeft` false)
        (goto _label :!via `Reset`)))
    (else
      (`/Engine/EditorBlueprintResources/StandardMacros.DoOnce` false :!label _label_2
        (:`Completed`
          (`KismetSystemLibrary.MoveComponentTo` _ashoo_flower (`self.LocationLeft`) (struct) false false _timetodestination)
          (`KismetSystemLibrary.Delay` (`self.Wait`))
          (set `self.isLeft` true)
          (goto _label_2 :!via `Reset`))))))

(fn `UserConstructionScript`)