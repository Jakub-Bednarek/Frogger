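; BP_JumpLily is a lily jump pad in Frogger Level 6 that bounces the player character upward on contact.
; An overlap with BP_ThirdPersonCharacter_Child launches it vertically with a force scaled by JumpPower, overriding only Z velocity, and plays a sound.
; A timeline restarts on each bounce, animating the flower mesh's vertical scale relative to the scale cached at BeginPlay.
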(event `self.ReceiveBeginPlay`
  (set `self.ScaleZ` (`SceneComponent.K2_GetComponentScale` (`self.ashoo_flower`))))

(event `self.ReceiveActorBeginOverlap`
  (params (OtherActor :type "Actor Object Reference"))
  (bind _asbp_third_person_character_child (cast `/Game/Frogger/Level_6_Content/Blueprints/BP_ThirdPersonCharacter_Child` OtherActor))
  (`Character.LaunchCharacter` _asbp_third_person_character_child (`KismetMathLibrary.MakeVector` 0.0 0.0 (* 500.0 (`self.JumpPower`))) false true)
  (`AudioComponent.Play` (`self.Audio`) 0.0)
  (bind (_direction _scale) (`Timeline|Animation` :!via `PlayFromStart`)
    (:`Update`
      (`SceneComponent.SetWorldScale3D` (`self.ashoo_flower`) (`KismetMathLibrary.MakeVector` (.x (`self.ScaleZ`)) (.y (`self.ScaleZ`)) (* _scale (.z (`self.ScaleZ`))))))))

(fn `UserConstructionScript`)