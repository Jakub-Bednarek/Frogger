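; Breakable lily pad actor for Frogger Level 6 that temporarily disappears after being stepped on.
; Any actor overlap starts a timer of BreakingTime that calls Break, which hides the AshooFlower component with its children and disables its collision.
; Break then schedules BringBack one second later, restoring visibility and query-and-physics collision.
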(event `self.ReceiveBeginPlay`)

(event `self.ReceiveActorBeginOverlap`
  (params (OtherActor :type "Actor Object Reference"))
  (`KismetSystemLibrary.K2_SetTimer` null "Break" (`self.BreakingTime`)))

(event `self.ReceiveTick`
  (params (DeltaSeconds :type "Float (single-precision)")))

(fn `Break`
  (bind _ashoo_flower (`self.ashoo_flower`))
  (`SceneComponent.SetVisibility` _ashoo_flower false true)
  (`PrimitiveComponent.SetCollisionEnabled` _ashoo_flower "NoCollision")
  (`KismetSystemLibrary.K2_SetTimer` null "BringBack" 1.0))

(fn `BringBack`
  (bind _ashoo_flower (`self.ashoo_flower`))
  (`SceneComponent.SetVisibility` _ashoo_flower true true)
  (`PrimitiveComponent.SetCollisionEnabled` _ashoo_flower "QueryAndPhysics"))

(fn `UserConstructionScript`)