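; Wasp enemy character for Frogger Level 6 that turns toward the player and attacks on detection.
; Tick smoothly rotates it to face the player and sets the attack flag on ABP_Wasp, which also holds the hit and dead states.
; DetectPlayer extends the parent check, returning false while hit or dead.
; Hit ignores damage during a hit reaction, otherwise reduces Health, and at zero flags death and destroys the actor after a delay.
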(event `self.ReceiveTick`
  (params (DeltaSeconds :type "Float (single-precision)"))
  (`parent.ReceiveTick` DeltaSeconds)
  (bind _detect (`self.DetectPlayer`))
  (bind _asabp_wasp (cast `/Game/Frogger/Level_6_Content/Animation/ABP_Wasp` (`SkeletalMeshComponent.GetAnimInstance` (`self.Mesh`))))
  (if _detect
    (`self.K2_SetActorRotation` (`KismetMathLibrary.RInterpTo` (`self.K2_GetActorRotation`) (`KismetMathLibrary.FindLookAtRotation` (`self.K2_GetActorLocation`) (`self.K2_GetActorLocation` (`GameplayStatics.GetPlayerCharacter` 0))) DeltaSeconds 9.0))
    (set `/Game/Frogger/Level_6_Content/Animation/ABP_Wasp.isAttacking` true _asabp_wasp)
    (else
      (set `/Game/Frogger/Level_6_Content/Animation/ABP_Wasp.isAttacking` false _asabp_wasp))))

(event `self.Hit`
  (params (Damage :type "Float (double-precision)"))
  (bind _asabp_wasp (cast `/Game/Frogger/Level_6_Content/Animation/ABP_Wasp` (`SkeletalMeshComponent.GetAnimInstance` (`self.Mesh`))))
  (if (not (`/Game/Frogger/Level_6_Content/Animation/ABP_Wasp.isHit` _asabp_wasp))
    (bind _output_get (set `self.Health` (- (`self.Health`) Damage)))
    (if (<= _output_get 0.0)
      (set `/Game/Frogger/Level_6_Content/Animation/ABP_Wasp.isDead` true _asabp_wasp)
      (`KismetSystemLibrary.Delay` 10.0)
      (`self.K2_DestroyActor`)
      (else
        (set `/Game/Frogger/Level_6_Content/Animation/ABP_Wasp.isHit` true _asabp_wasp)))))

(fn `DetectPlayer`
  (returns (Detect :type Boolean))
  (bind _detect (`parent.DetectPlayer`))
  (bind _asabp_wasp (cast `/Game/Frogger/Level_6_Content/Animation/ABP_Wasp` (`SkeletalMeshComponent.GetAnimInstance` (`self.Mesh`))))
  (return (and (not (or (`/Game/Frogger/Level_6_Content/Animation/ABP_Wasp.isHit` _asabp_wasp) (`/Game/Frogger/Level_6_Content/Animation/ABP_Wasp.isDead` _asabp_wasp))) _detect)))

(fn `UserConstructionScript`
  (`parent.UserConstructionScript`))