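; BP_Camera is a camera actor for Frogger Level 6 that follows the player vertically.
; It caches the Camera component's relative location on BeginPlay as the rest position.
; Each tick, while the player pawn's world Z exceeds a fixed threshold, MoveComponentTo moves the camera's relative Z to that value, keeping X and Y.
; Otherwise, it eases the camera back to the cached position.
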(event `self.ReceiveBeginPlay`
  (set `self.CameraLocation` (.location (`SceneComponent.GetRelativeTransform` (`self.Camera`)))))

(event `self.ReceiveTick`
  (params (DeltaSeconds :type "Float (single-precision)"))
  (bind _camera (`self.Camera`))
  (bind _cameralocation (`self.CameraLocation`))
  (bind _z (.z (.location (`self.GetTransform` (`GameplayStatics.GetPlayerPawn` 0)))))
  (if (> _z 200.0)
    (`KismetSystemLibrary.MoveComponentTo` _camera (`KismetMathLibrary.MakeVector` (.x _cameralocation) (.y _cameralocation) _z))
    (else
      (`KismetSystemLibrary.MoveComponentTo` _camera _cameralocation (struct) false false 0.5))))

(fn `UserConstructionScript`)