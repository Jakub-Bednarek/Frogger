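; BP_Fly is a fly actor that rises while swaying sideways and awards score through BP_FrogTheFroggerGameMode when something overlaps it.
; Tick re-arms the move flag and plays a timeline whose Flow track drives sideways offset, alongside frame-time-scaled climb.
; At target height, it asks a valid spawner for a new fly, then destroys itself.
; An overlap destroys it after a short delay, then adds a point.
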(event `self.ReceiveTick`
  (params (DeltaSeconds :type "Float (single-precision)"))
  (bind _returnvalue (+ (.z (`self.BaseLocation`)) (* (`self.FlySpeed`) (`GameplayStatics.GetWorldDeltaSeconds`))))
  (bind _output_get (set `self.bCanMoveUp` true))
  (if _output_get
    (set `self.BaseLocation` (`self.K2_GetActorLocation`))
    (bind (_direction _flow) (`Timeline|Timeline`)
      (:`Update`
        (`self.K2_SetActorLocation` (`KismetMathLibrary.MakeVector` (.x (`self.BaseLocation`)) (+ (.y (`self.BaseLocation`)) (* (`self.SideSpeed`) _flow)) _returnvalue))
        (if (>= _returnvalue (`self.TargetHeight`))
          (set `self.bCanMoveUp` false)
          (`/Engine/EditorBlueprintResources/StandardMacros.IsValid` (`self.FlySpawnerRef`)
            (:`Is Valid`
              (`/Game/Frogger/Level_4_Content/Content/BluePrints/BP_FlySpawner.SpawnFly` (`self.FlySpawnerRef`))
              (`self.K2_DestroyActor`))))))))

(event `self.Collider.OnComponentBeginOverlap`
  (params (OverlappedComponent :type "PrimitiveComponent Object Reference") (OtherActor :type "Actor Object Reference") (OtherComp :type "PrimitiveComponent Object Reference") (OtherBodyIndex :type Integer) (bFromSweep :type Boolean) (SweepResult :type "HitResult Structure (by ref)"))
  (`KismetSystemLibrary.PrintString` "Hit")
  (`KismetSystemLibrary.Delay` 0.2)
  (`self.K2_DestroyActor`)
  (bind _asbp_frog_game_mode (cast `/Game/Frogger/Level_4_Content/Content/ThirdPerson/Blueprints/BP_FrogTheFroggerGameMode` (`GameplayStatics.GetGameMode`)))
  (`/Game/Frogger/Level_4_Content/Content/ThirdPerson/Blueprints/BP_FrogTheFroggerGameMode.AddScore` _asbp_frog_game_mode 1))

(fn `UserConstructionScript`)