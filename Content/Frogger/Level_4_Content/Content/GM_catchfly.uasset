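; Game mode for a fly-catching game that tracks the score and triggers the win screen.
; BeginPlay sets game-only input and hides the mouse cursor.
; AddScore accumulates points and calls ShowWinScreen once the score reaches WinScore.
; ShowWinScreen adds WBP_WinScreen to the viewport, switches to UI-only input with the cursor still hidden, and disables input on the player character.
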(event `self.ReceiveBeginPlay`
  (bind _returnvalue (`PlayerState.GetPlayerController` (`Pawn.PlayerState` (`GameplayStatics.GetPlayerCharacter` 0))))
  (`WidgetBlueprintLibrary.SetInputMode_GameOnly` _returnvalue)
  (set `PlayerController.bShowMouseCursor` false _returnvalue))

(fn `AddScore`
  (params (Points :type Integer))
  (set `self.Score` (+ Points (`self.Score`)))
  (if (>= (`self.Score`) (`self.WinScore`))
    (`self.ShowWinScreen`)))

(fn `ShowWinScreen`
  (bind _returnvalue (`GameplayStatics.GetPlayerController` 0))
  (bind _returnvalue_2 (`|CreateWidget` "/Game/Frogger/Level_4_Content/Content/WBP_WinScreen.WBP_WinScreen_C" _returnvalue))
  (`UserWidget.AddToViewport` _returnvalue_2 0)
  (`WidgetBlueprintLibrary.SetInputMode_UIOnlyEx` _returnvalue _returnvalue_2)
  (set `PlayerController.bShowMouseCursor` false _returnvalue)
  (`self.DisableInput` (`GameplayStatics.GetPlayerCharacter` 0) _returnvalue))

(fn `UserConstructionScript`)